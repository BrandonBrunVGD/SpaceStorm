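; BP_Asteroid is a falling enemy sprite with randomized look, scale and spin direction that bullets can destroy.
; Tick spins it, moves it down world Z and checks health; at zero it awards player score and may drop a shield, heart or double-shoot power-up.
; Bullet overlaps reduce health shown on a widget bar hidden at full health, while touching the death wall or character destroys it without score or drop.
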(event `self.ReceiveBeginPlay`
  (`self.RanAsteroid`)
  (`self.RanScale`)
  (if (`KismetMathLibrary.RandomBool`)
    (set `self.SpinDirection` -0.5)
    (else
      (set `self.SpinDirection` 0.5))))

(event `RanAsteroid`
  (bind _asteroid (`self.Asteroid`))
  (switch `int` (`KismetMathLibrary.RandomIntegerInRange` 0 (- (`self.TotalAsteroids`) 1))
    (:`Default`
      (`PaperSpriteComponent.SetSprite` _asteroid "/Game/Blueprints/Asteroids/Asteroid_1_Sprite.Asteroid_1_Sprite" :!label _label))
    (:`0`
      (goto _label))
    (:`1`
      (`PaperSpriteComponent.SetSprite` _asteroid "/Game/Blueprints/Asteroids/Asteroid_2_Sprite.Asteroid_2_Sprite"))
    (:`2`
      (`PaperSpriteComponent.SetSprite` _asteroid "/Game/Blueprints/Asteroids/Asteroid_3_Sprite.Asteroid_3_Sprite"))))

(event `RanScale`
  (bind (_returnvalue_location _returnvalue_rotation _returnvalue_scale) (`KismetMathLibrary.BreakTransform` (`self.GetTransform`)))
  (`self.K2_SetActorTransform` (`KismetMathLibrary.MakeTransform` _returnvalue_location _returnvalue_rotation (* _returnvalue_scale (`KismetMathLibrary.RandomFloatInRange` 0.5 2.0)))))

(event `self.ReceiveActorBeginOverlap`
  (params (OtherActor :type "Actor Object Reference"))
  (cast `/Game/Blueprints/Bullet/BP_Bullet` OtherActor
    (:`then`
      (set `self.Health` (- (`self.Health`) 1.0))
      (`self.HandleHealthBar`))
    (:`CastFailed`
      (cast `/Game/Blueprints/Bounds/BP_DeathWall` OtherActor
        (:`then`
          _)
        (:`CastFailed`
          (cast `/Game/Ship/BP_Character` OtherActor)))
      (`self.K2_DestroyActor`))))

(event `self.ReceiveTick`
  (params (DeltaSeconds :type "Float (single-precision)"))
  (`self.HandleHealthBar`)
  (`SceneComponent.K2_AddLocalRotation` (`self.Asteroid`) (`KismetMathLibrary.MakeRotator` 0.0 (`self.SpinDirection`)) false false)
  (`self.K2_AddActorWorldOffset` (0.0 0.0 -0.5))
  (if (<= (`self.Health`) 0.0)
    (`self.SpawnPowerUp`)
    (bind _asbp_character (cast `/Game/Ship/BP_Character` (`GameplayStatics.GetPlayerPawn` 0)))
    (set `/Game/Ship/BP_Character.Score` (+ (`/Game/Ship/BP_Character.Score` _asbp_character) 10) _asbp_character)
    (`self.K2_DestroyActor`)))

(event `SpawnPowerUp`
  (bind (_returnvalue_location _returnvalue_rotation) (`KismetMathLibrary.BreakTransform` (`self.GetTransform`)))
  (if (== (`KismetMathLibrary.RandomIntegerInRange` 1 3) 1)
    (switch `int` (`KismetMathLibrary.RandomIntegerInRange` 0 2)
      (:`Default`
        (`|SpawnActorFromClass` "/Game/Blueprints/PowerUps/BP_ShieldPU.BP_ShieldPU_C" (`KismetMathLibrary.MakeTransform` _returnvalue_location _returnvalue_rotation) "Undefined" "MultiplyWithRoot" null null :!label _label_2))
      (:`0`
        (goto _label_2))
      (:`1`
        (`|SpawnActorFromClass` "/Game/Blueprints/PowerUps/BP_HeartPU.BP_HeartPU_C" (`KismetMathLibrary.MakeTransform` _returnvalue_location _returnvalue_rotation) "Undefined" "MultiplyWithRoot" null null))
      (:`2`
        (`|SpawnActorFromClass` "/Game/Blueprints/PowerUps/BP_DoubleShootPU.BP_DoubleShootPU_C" (`KismetMathLibrary.MakeTransform` _returnvalue_location _returnvalue_rotation) "Undefined" "MultiplyWithRoot" null null)))))

(event `HandleHealthBar`
  (bind _health (`self.Health`))
  (bind _maxhealth (`self.MaxHealth`))
  (bind _returnvalue (`WidgetComponent.GetWidget` (`self.HealthBar`)))
  (bind _aswidget_ehealth_bar (cast `/Game/Blueprints/Enemies/Widget_EHealthBar` _returnvalue))
  (`ProgressBar.SetPercent` (`/Game/Blueprints/Enemies/Widget_EHealthBar.HealthBar` _aswidget_ehealth_bar) (/ _health _maxhealth))
  (if (== _health _maxhealth)
    (set `Widget.Visibility` "Hidden" _returnvalue)
    (else
      (set `Widget.Visibility` "Visible" _returnvalue))))

(fn `UserConstructionScript`)