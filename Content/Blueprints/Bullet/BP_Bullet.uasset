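; BP_Bullet is a laser projectile that tints its sprite blue and plays a shot sound on BeginPlay.
; Tick moves it along world +Z by a fixed offset per frame, without sweep or delta-time scaling.
; On overlap, cast checks destroy it silently at death walls, or with a blue-glow hit effect and impact sound on asteroids, enemies, rockets and boss bodies.
; It applies no damage itself.
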(event `self.ReceiveBeginPlay`
  (set `self.BulletColor` (`KismetMathLibrary.Conv_LinearColorToColor` (struct :`G` 0.088777 :`B` 1.0 :`A` 1.0)))
  (`PaperSpriteComponent.SetSpriteColor` (`self.PaperSprite`) (`KismetMathLibrary.Conv_ColorToLinearColor` (`self.BulletColor`)))
  (`GameplayStatics.PlaySound2D` "/Game/SFX/LaserShoot.LaserShoot" 1.0 1.0 0.0 null null))

(event `self.ReceiveActorBeginOverlap`
  (params (OtherActor :type "Actor Object Reference"))
  (cast `/Game/Blueprints/Bounds/BP_DeathWall` OtherActor
    (:`then`
      _)
    (:`CastFailed`
      (cast `/Game/Blueprints/Asteroids/BP_Asteroid` OtherActor
        (:`then`
          _)
        (:`CastFailed`
          (cast `/Game/Blueprints/Enemies/UFO/BP_Enemy` OtherActor
            (:`then`
              _)
            (:`CastFailed`
              (cast `/Game/Blueprints/Enemies/Rocket/BP_Rocket` OtherActor
                (:`then`
                  _)
                (:`CastFailed`
                  (cast `/Game/Blueprints/Enemies/Boss/BP_BossBody` OtherActor)))))))
      (`|SpawnActorFromClass` "/Game/FX/LaserHitEffect.LaserHitEffect_C" (`self.GetTransform`) "Undefined" "MultiplyWithRoot" null (struct :`B` 255 :`A` 255) "/Game/FX/Sprites/M_HitBlueGlow.M_HitBlueGlow" null)
      (`GameplayStatics.PlaySound2D` "/Game/SFX/LaserImpact.LaserImpact" 1.0 1.0 0.0 null null)))
  (`self.K2_DestroyActor`))

(event `self.ReceiveTick`
  (params (DeltaSeconds :type "Float (single-precision)"))
  (`self.K2_AddActorWorldOffset` (0.0 0.0 1.0)))

(fn `UserConstructionScript`)