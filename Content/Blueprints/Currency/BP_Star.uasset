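; BP_Star is a collectible currency pickup that randomly spawns as a common small star or a rarer, larger, higher-value one with its own sprite and glow material.
; On BeginPlay it stops BP_Pet following and sends it to the star's location.
; Overlap by either the character or the pet credits the player's BP_Character with the stars and destroys the actor.
; Tick bobs it vertically, using Delays to flip direction.
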(event `self.ReceiveBeginPlay`
  (bind (_returnvalue_location _returnvalue_rotation) (`KismetMathLibrary.BreakTransform` (`self.GetTransform`)))
  (bind _papersprite (`self.PaperSprite`))
  (bind _papersprite1 (`self.PaperSprite1`))
  (bind _spawnchance (`self.SpawnChance`))
  (if (< (`KismetMathLibrary.RandomIntegerInRange` 1 _spawnchance) _spawnchance)
    (`PaperSpriteComponent.SetSprite` _papersprite "/Game/Blueprints/Currency/Star_Small_Sprite.Star_Small_Sprite")
    (set `self.StarsToAdd` 1)
    (`PrimitiveComponent.SetMaterial` _papersprite1 0 "/Game/Blueprints/Currency/M_SmallStarGlow.M_SmallStarGlow")
    (else
      (`PaperSpriteComponent.SetSprite` _papersprite "/Game/Blueprints/Currency/Star_Big_Sprite.Star_Big_Sprite")
      (set `self.StarsToAdd` 5)
      (`PrimitiveComponent.SetMaterial` _papersprite1 0 "/Game/Blueprints/Currency/M_BigStarGlow1.M_BigStarGlow1")
      (`self.K2_SetActorTransform` (`KismetMathLibrary.MakeTransform` _returnvalue_location _returnvalue_rotation (2.0 2.0 2.0)))))
  (bind _returnvalue (`GameplayStatics.GetActorOfClass` "/Game/Blueprints/Pets/BP_Pet.BP_Pet_C"))
  (bind _output_get (set `self.As BP Pet` _returnvalue))
  (set `/Game/Blueprints/Pets/BP_Pet.IsFollowing` false _output_get)
  (set `/Game/Blueprints/Pets/BP_Pet.PosB` (`self.K2_GetActorLocation`) _output_get)
  (`/Game/Blueprints/Pets/BP_Pet.MoveToStar` _output_get))

(event `self.ReceiveActorBeginOverlap`
  (params (OtherActor :type "Actor Object Reference"))
  (cast `/Game/Ship/BP_Character` OtherActor
    (:`then`
      _)
    (:`CastFailed`
      (bind _asbp_pet (cast `/Game/Blueprints/Pets/BP_Pet` OtherActor))
      (set `self.As BP Pet` _asbp_pet)
      (bind _asbp_character (cast `/Game/Ship/BP_Character` (`GameplayStatics.GetPlayerPawn` 0)))))
  (set `/Game/Ship/BP_Character.StarsAdded` (`self.StarsToAdd`) _asbp_character)
  (`/Game/Ship/BP_Character.AddStars` _asbp_character 0)
  (`self.K2_DestroyActor`))

(event `self.ReceiveTick`
  (params (DeltaSeconds :type "Float (single-precision)"))
  (if (`self.UpDown`)
    (`self.K2_AddActorWorldOffset` (0.0 0.0 -0.1))
    (`KismetSystemLibrary.Delay` 0.5)
    (set `self.UpDown` false)
    (else
      (`self.K2_AddActorWorldOffset` (0.0 0.0 0.1))
      (`KismetSystemLibrary.Delay` 0.5)
      (set `self.UpDown` true))))

(fn `UserConstructionScript`)