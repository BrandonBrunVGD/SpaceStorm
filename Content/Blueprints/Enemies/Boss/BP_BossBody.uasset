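; Boss enemy body that descends to a height threshold, then patrols side to side with a Delay-toggled vertical bob.
; Tick drives movement using fixed per-frame offsets; overlaps with bound actors flip direction and bullet overlaps reduce Health.
; The widget health bar updates only during descent, hidden at full health.
; It switches off the rocket and enemy spawners on BeginPlay and again at zero Health, when it destroys itself.
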(event `self.ReceiveBeginPlay`
  (bind _returnvalue (`GameplayStatics.GetActorOfClass` "/Game/Blueprints/Enemies/Rocket/BP_RocketSpawner.BP_RocketSpawner_C"))
  (bind _output_get (set `self.BPRocket` _returnvalue))
  (set `/Game/Blueprints/Enemies/Rocket/BP_RocketSpawner.ShouldSpawn` false _output_get)
  (bind _returnvalue_2 (`GameplayStatics.GetActorOfClass` "/Game/Blueprints/Enemies/UFO/BP_EnemySpawner.BP_EnemySpawner_C"))
  (bind _output_get_2 (set `self.BPEnemySpawner` _returnvalue_2))
  (set `/Game/Blueprints/Enemies/UFO/BP_EnemySpawner.ShouldSpawn` false _output_get_2))

(event `self.ReceiveActorBeginOverlap`
  (params (OtherActor :type "Actor Object Reference"))
  (cast `/Game/Blueprints/Bounds/BP_BoundsRight` OtherActor
    (:`then`
      (set `self.RIght` false))
    (:`CastFailed`
      (cast `/Game/Blueprints/Bounds/BP_BoundsLeft` OtherActor
        (:`then`
          (set `self.RIght` true))
        (:`CastFailed`
          (cast `/Game/Blueprints/Bullet/BP_Bullet` OtherActor)
          (set `self.Health` (- (`self.Health`) 1.0)))))))

(event `MoveLeftRight`
  (bind _movespeed (`self.MoveSpeed`))
  (if (`self.RIght`)
    (`self.K2_AddActorWorldOffset` (`KismetMathLibrary.MakeVector` 0.0 (* _movespeed -1.0)))
    (else
      (`self.K2_AddActorWorldOffset` (`KismetMathLibrary.MakeVector` 0.0 _movespeed)))))

(event `self.ReceiveTick`
  (params (DeltaSeconds :type "Float (single-precision)"))
  (bind (_returnvalue_x _returnvalue_y _returnvalue_z) (`KismetMathLibrary.BreakVector` (`self.K2_GetActorLocation`)))
  (if (<= (`self.Health`) 0.0)
    (set `/Game/Blueprints/Enemies/Rocket/BP_RocketSpawner.ShouldSpawn` false (`self.BPRocket`))
    (set `/Game/Blueprints/Enemies/UFO/BP_EnemySpawner.ShouldSpawn` false (`self.BPEnemySpawner`))
    (`self.K2_DestroyActor`)
    (elif (> _returnvalue_z 600.0)
      (`self.K2_AddActorWorldOffset` (0.0 0.0 -0.1))
      (`self.HandleHealthBar`)
      (else
        (`self.MoveLeftRight`)
        (`self.MoveUpDown`)))))

(event `HandleHealthBar`
  (bind _health (`self.Health`))
  (bind _maxhealth (`self.MaxHealth`))
  (bind _returnvalue (`WidgetComponent.GetWidget` (`self.HealthBar`)))
  (bind _aswidget_ehealth_bar (cast `/Game/Blueprints/Enemies/Widget_EHealthBar` _returnvalue))
  (`ProgressBar.SetPercent` (`/Game/Blueprints/Enemies/Widget_EHealthBar.HealthBar` _aswidget_ehealth_bar) (/ _health _maxhealth))
  (if (== _health _maxhealth)
    (set `Widget.Visibility` "Hidden" _returnvalue)
    (else
      (set `Widget.Visibility` "Visible" _returnvalue))))

(event `MoveUpDown`
  (if (`self.Up`)
    (`self.K2_AddActorWorldOffset` (0.0 0.0 -0.1))
    (`KismetSystemLibrary.Delay` 0.5)
    (set `self.Up` false)
    (else
      (`self.K2_AddActorWorldOffset` (0.0 0.0 0.1))
      (`KismetSystemLibrary.Delay` 0.5)
      (set `self.Up` true))))

(fn `UserConstructionScript`)