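; BP_BossGun is a boss weapon that tracks the player and periodically fires rockets.
; It caches the player's BP_Character on BeginPlay, then each Tick turns its local Y axis toward that character, keeping world up as reference.
; Tick also calls Shoot, where a random 5–10 second Delay absorbs repeat calls and acts as the fire timer before spawning BP_Rocket with the gun's location and rotation.
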(event `self.ReceiveBeginPlay`
  (bind _asbp_character (cast `/Game/Ship/BP_Character` (`GameplayStatics.GetPlayerPawn` 0)))
  (set `self.As BP Character` _asbp_character)
  (`self.FacePlayer`))

(event `self.ReceiveTick`
  (params (DeltaSeconds :type "Float (single-precision)"))
  (`self.Shoot`)
  (`self.FacePlayer`))

(event `Shoot`
  (bind (_returnvalue_location _returnvalue_rotation) (`KismetMathLibrary.BreakTransform` (`self.GetTransform`)))
  (`KismetSystemLibrary.Delay` (`KismetMathLibrary.RandomFloatInRange` 5.0 10.0))
  (`|SpawnActorFromClass` "/Game/Blueprints/Enemies/Rocket/BP_Rocket.BP_Rocket_C" (`KismetMathLibrary.MakeTransform` _returnvalue_location _returnvalue_rotation) "Undefined" "MultiplyWithRoot" null null))

(event `FacePlayer`
  (bind (_returnvalue_roll _returnvalue_pitch _returnvalue_yaw) (`KismetMathLibrary.BreakRotator` (`KismetMathLibrary.MakeRotFromYZ` (- (`self.K2_GetActorLocation` (`self.As BP Character`)) (`self.K2_GetActorLocation`)) (`KismetMathLibrary.Vector_Up`))))
  (`self.K2_SetActorRotation` (`KismetMathLibrary.MakeRotator` _returnvalue_roll _returnvalue_pitch _returnvalue_yaw) true))

(fn `UserConstructionScript`)