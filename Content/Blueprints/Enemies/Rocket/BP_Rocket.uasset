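; Homing enemy rocket that chases the player character and is destroyed on contact with the player or a bullet.
; Each tick it steps toward the cached player by a fixed speed on world Y (MoveX) and Z (MoveY), then rotates its Y axis to face them.
; Overlapping either target spawns a red laser hit effect at its location before destroying it, with no damage applied in this graph.
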(event `self.ReceiveBeginPlay`
  (bind _asbp_character (cast `/Game/Ship/BP_Character` (`GameplayStatics.GetPlayerPawn` 0)))
  (set `self.As BP Character` _asbp_character)
  (`self.FacePlayer`))

(event `self.ReceiveActorBeginOverlap`
  (params (OtherActor :type "Actor Object Reference"))
  (bind _returnvalue (`self.GetTransform`))
  (cast `/Game/Ship/BP_Character` OtherActor
    (:`then`
      _)
    (:`CastFailed`
      (cast `/Game/Blueprints/Bullet/BP_Bullet` OtherActor)))
  (bind _structout (setmembers `Color` :`StructRef` (`KismetMathLibrary.LinearColor_ToRGBE` (struct :`R` 1.0 :`A` 1.0))))
  (`|SpawnActorFromClass` "/Game/FX/LaserHitEffect.LaserHitEffect_C" (`KismetMathLibrary.MakeTransform` (`KismetMathLibrary.MakeVector` (.x (.location _returnvalue)) (.y (.location _returnvalue)) (.z (.location _returnvalue))) (struct :`Yaw` -90.0)) "Undefined" "MultiplyWithRoot" null _structout "/Game/FX/Sprites/M_HitRedGlow.M_HitRedGlow" null)
  (`self.K2_DestroyActor`))

(event `MoveY`
  (bind (_returnvalue_x _returnvalue_y _returnvalue_z) (`KismetMathLibrary.BreakVector` (`self.K2_GetActorLocation`)))
  (bind (_returnvalue_x_2 _returnvalue_y_2 _returnvalue_z_2) (`KismetMathLibrary.BreakVector` (`self.K2_GetActorLocation` (`self.As BP Character`))))
  ;[1 1 1] MoveRocketToPlayer
  (if (> _returnvalue_z _returnvalue_z_2)
    (`self.K2_AddActorWorldOffset` (`KismetMathLibrary.MakeVector` 0.0 0.0 (* (`self.MoveSpeed`) -1.0)))
    (elif (< _returnvalue_z _returnvalue_z_2)
      (`self.K2_AddActorWorldOffset` (`KismetMathLibrary.MakeVector` 0.0 0.0 (`self.MoveSpeed`))))))

(event `self.ReceiveTick`
  (params (DeltaSeconds :type "Float (single-precision)"))
  (`self.MoveX`)
  (`self.MoveY`)
  (`self.FacePlayer`))

(event `MoveX`
  (bind (_returnvalue_x _returnvalue_y) (`KismetMathLibrary.BreakVector` (`self.K2_GetActorLocation`)))
  (bind (_returnvalue_x_2 _returnvalue_y_2) (`KismetMathLibrary.BreakVector` (`self.K2_GetActorLocation` (`self.As BP Character`))))
  ;[1 1 1] MoveRocketToPlayer
  (if (> _returnvalue_y _returnvalue_y_2)
    (`self.K2_AddActorWorldOffset` (`KismetMathLibrary.MakeVector` 0.0 (* (`self.MoveSpeed`) -1.0)))
    (elif (< _returnvalue_y _returnvalue_y_2)
      (`self.K2_AddActorWorldOffset` (`KismetMathLibrary.MakeVector` 0.0 (`self.MoveSpeed`))))))

(event `FacePlayer`
  (bind (_returnvalue_roll _returnvalue_pitch _returnvalue_yaw) (`KismetMathLibrary.BreakRotator` (`KismetMathLibrary.MakeRotFromYZ` (- (`self.K2_GetActorLocation` (`self.As BP Character`)) (`self.K2_GetActorLocation`)) (`KismetMathLibrary.Vector_Up`))))
  (`self.K2_SetActorRotation` (`KismetMathLibrary.MakeRotator` _returnvalue_roll _returnvalue_pitch _returnvalue_yaw) true))

(fn `UserConstructionScript`)