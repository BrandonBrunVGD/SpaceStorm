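; Enemy rocket spawner actor that repeatedly launches rockets, each preceded by a warning, while ShouldSpawn is true.
; Tick drives chained Delays: a random wait spawns BP_Warning at fixed X and Z, then BP_Rocket follows two seconds later from the spawner's X and Z.
; Both share a random Y offset from the spawner, rolled only once at BeginPlay.
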(event `self.ReceiveBeginPlay`
  (set `self.RandomPOS` (`KismetMathLibrary.RandomFloatInRange` -500.0 500.0)))

(event `self.ReceiveTick`
  (params (DeltaSeconds :type "Float (single-precision)"))
  (bind _returnvalue (`self.GetTransform`))
  (bind _returnvalue_2 (+ (.y (.location _returnvalue)) (`self.RandomPOS`)))
  (if (`self.ShouldSpawn`)
    (`KismetSystemLibrary.Delay` (`KismetMathLibrary.RandomFloatInRange` 10.0 15.0))
    (`|SpawnActorFromClass` "/Game/Blueprints/Enemies/Rocket/BP_Warning.BP_Warning_C" (`KismetMathLibrary.MakeTransform` (`KismetMathLibrary.MakeVector` 600.0 _returnvalue_2 625.0) (.rotation _returnvalue) (.scale _returnvalue)) "Undefined" "MultiplyWithRoot" null null)
    (`KismetSystemLibrary.Delay` 2.0)
    (`|SpawnActorFromClass` "/Game/Blueprints/Enemies/Rocket/BP_Rocket.BP_Rocket_C" (`KismetMathLibrary.MakeTransform` (`KismetMathLibrary.MakeVector` (.x (.location _returnvalue)) _returnvalue_2 (.z (.location _returnvalue))) (struct) (.scale _returnvalue)) "Undefined" "MultiplyWithRoot" null null)))

(fn `UserConstructionScript`)