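; UFO enemy that descends to a set height, then patrols sideways with a slight bob, reversing at left and right bound actors.
; Bullet overlaps reduce Health, shown on a widget bar that is hidden at full health.
; Tick drives movement, bar updates and death, using retrigger-ignoring Delays to time bobbing and randomly spaced shots.
; Death awards score to the player, spawns a star, stops the hover sound and destroys the actor.
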(event `self.ReceiveBeginPlay`
  (bind _returnvalue (`GameplayStatics.SpawnSound2D` "/Game/SFX/UFOHover.UFOHover" 1.0 1.0 0.0 null))
  (set `self.UFOHoverSound` _returnvalue))

(event `self.ReceiveActorBeginOverlap`
  (params (OtherActor :type "Actor Object Reference"))
  (cast `/Game/Blueprints/Bullet/BP_Bullet` OtherActor
    (:`then`
      (set `self.Health` (- (`self.Health`) 1.0)))
    (:`CastFailed`
      (cast `/Game/Blueprints/Bounds/BP_BoundsRight` OtherActor
        (:`then`
          (set `self.RIght` false))
        (:`CastFailed`
          (cast `/Game/Blueprints/Bounds/BP_BoundsLeft` OtherActor)
          (set `self.RIght` true))))))

(event `self.ReceiveTick`
  (params (DeltaSeconds :type "Float (single-precision)"))
  (bind (_returnvalue_location _returnvalue_rotation) (`KismetMathLibrary.BreakTransform` (`self.GetTransform`)))
  (bind (_returnvalue_x _returnvalue_y _returnvalue_z) (`KismetMathLibrary.BreakVector` (`SceneComponent.K2_GetComponentLocation` (`self.PaperSprite`))))
  (`self.Shoot`)
  (`self.HandleHealthBar`)
  (if (<= (`self.Health`) 0.0)
    (bind _asbp_character (cast `/Game/Ship/BP_Character` (`GameplayStatics.GetPlayerPawn` 0)))
    (set `/Game/Ship/BP_Character.Score` (+ (`/Game/Ship/BP_Character.Score` _asbp_character) 30) _asbp_character)
    (`|SpawnActorFromClass` "/Game/Blueprints/Currency/BP_Star.BP_Star_C" (`KismetMathLibrary.MakeTransform` _returnvalue_location _returnvalue_rotation) "Undefined" "MultiplyWithRoot" null null)
    (`AudioComponent.Stop` (`self.UFOHoverSound`))
    (`self.K2_DestroyActor`)
    (elif (> _returnvalue_z 550.0)
      (`self.K2_AddActorWorldOffset` (0.0 0.0 -1.0))
      (else
        (`self.Move`)
        (`self.MoveUpDown`)))))

(event `Move`
  (bind _movespeed (`self.MoveSpeed`))
  (if (`self.RIght`)
    (`self.K2_AddActorWorldOffset` (`KismetMathLibrary.MakeVector` 0.0 (* _movespeed -1.0)))
    (else
      (`self.K2_AddActorWorldOffset` (`KismetMathLibrary.MakeVector` 0.0 _movespeed)))))

(event `HandleHealthBar`
  (bind _health (`self.Health`))
  (bind _maxhealth (`self.MaxHealth`))
  (bind _returnvalue (`WidgetComponent.GetWidget` (`self.HealthBar`)))
  (bind _aswidget_ehealth_bar (cast `/Game/Blueprints/Enemies/Widget_EHealthBar` _returnvalue))
  (`ProgressBar.SetPercent` (`/Game/Blueprints/Enemies/Widget_EHealthBar.HealthBar` _aswidget_ehealth_bar) (/ _health _maxhealth))
  (if (== _health _maxhealth)
    (set `Widget.Visibility` "Hidden" _returnvalue)
    (else
      (set `Widget.Visibility` "Visible" _returnvalue))))

(event `MoveUpDown`
  (if (`self.Up`)
    (`self.K2_AddActorWorldOffset` (0.0 0.0 -0.1))
    (`KismetSystemLibrary.Delay` 0.5)
    (set `self.Up` false)
    (else
      (`self.K2_AddActorWorldOffset` (0.0 0.0 0.1))
      (`KismetSystemLibrary.Delay` 0.5)
      (set `self.Up` true))))

(event `Shoot`
  (bind (_returnvalue_location _returnvalue_rotation) (`KismetMathLibrary.BreakTransform` (`self.GetTransform`)))
  (`KismetSystemLibrary.Delay` (`KismetMathLibrary.RandomFloatInRange` 2.0 5.0))
  (`|SpawnActorFromClass` "/Game/Blueprints/Enemies/BP_EBullet.BP_EBullet_C" (`KismetMathLibrary.MakeTransform` _returnvalue_location _returnvalue_rotation) "Undefined" "MultiplyWithRoot" null null))

(fn `UserConstructionScript`)