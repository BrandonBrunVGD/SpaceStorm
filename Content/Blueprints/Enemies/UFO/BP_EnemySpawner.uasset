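; Enemy spawner Blueprint that spawns actors while ShouldSpawn is set and brings in BP_BossBody once game time reaches TimeToSpawnBoss.
; Tick drives everything, using Delay nodes to space regular spawns at random intervals and to count TimeInGame in seconds until StopTimer is set.
; Regular spawns get a random Y offset from the spawner.
; The boss spawns through a DoOnce at a fixed X, using the spawner's Y and Z.
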(event `self.ReceiveBeginPlay`)

(event `self.ReceiveTick`
  (params (DeltaSeconds :type "Float (single-precision)"))
  (bind _returnvalue (`self.GetTransform`))
  (`self.HandleBossSpawn`)
  (`self.Timer`)
  (if (`self.ShouldSpawn`)
    (`KismetSystemLibrary.Delay` (`KismetMathLibrary.RandomFloatInRange` 5.0 10.0))
    (`|SpawnActorFromClass` "/Game/Blueprints/Enemies/UFO/BP_Enemy.BP_Enemy_C" (`KismetMathLibrary.MakeTransform` (`KismetMathLibrary.MakeVector` (.x (.location _returnvalue)) (+ (.y (.location _returnvalue)) (`KismetMathLibrary.RandomFloatInRange` -500.0 500.0)) (.z (.location _returnvalue))) (.rotation _returnvalue) (.scale _returnvalue)) "Undefined" "MultiplyWithRoot" null null)))

(event `Timer`
  (if (not (`self.StopTimer`))
    (`KismetSystemLibrary.Delay` 1.0)
    (set `self.TimeInGame` (+ (`self.TimeInGame`) 1.0))))

(event `HandleBossSpawn`
  (bind _returnvalue (`self.GetTransform`))
  (if (>= (`self.TimeInGame`) (`self.TimeToSpawnBoss`))
    (`/Engine/EditorBlueprintResources/StandardMacros.DoOnce` false
      (:`Completed`
        (`|SpawnActorFromClass` "/Game/Blueprints/Enemies/Boss/BP_BossBody.BP_BossBody_C" (`KismetMathLibrary.MakeTransform` (`KismetMathLibrary.MakeVector` 380.0 (.y (.location _returnvalue)) (.z (.location _returnvalue))) (.rotation _returnvalue) (.scale _returnvalue)) "Undefined" "MultiplyWithRoot" null null)))))

(fn `UserConstructionScript`)