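; BP_Pet is a bird companion that flies out to fetch a star and brings it back to the player.
; MoveToStar plays a crow sound and lerps from an offset beside the player's live location to PosB on a timeline, then ReturnFromStar reverses a second timeline back.
; Overlapping a BP_Star shows the StarInMouth component.
; Finishing the return sets IsFollowing, which makes Tick hide that star.
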(event `self.ReceiveBeginPlay`
  (bind _asbp_enemy (cast `/Game/Blueprints/Enemies/UFO/BP_Enemy` (`self.BP_Enemy`)))
  (set `self.As BP Enemy` _asbp_enemy))

(event `self.ReceiveActorBeginOverlap`
  (params (OtherActor :type "Actor Object Reference"))
  (cast `/Game/Blueprints/Currency/BP_Star` OtherActor)
  (cast `/Game/Ship/BP_Character` (`GameplayStatics.GetPlayerPawn` 0))
  (`SceneComponent.SetVisibility` (`self.StarInMouth`) true true))

(event `MoveToStar`
  (bind (_returnvalue_x _returnvalue_y _returnvalue_z) (`KismetMathLibrary.BreakVector` (`self.K2_GetActorLocation` (`GameplayStatics.GetPlayerPawn` 0))))
  ;[1 1 1] Bird Goes and Gets the Star
  (`GameplayStatics.PlaySound2D` "/Game/SFX/CrowSound.CrowSound" 1.0 1.0 0.0 null null)
  (bind (_direction _curve) (`Timeline|Timeline` :!via `PlayFromStart`)
    (:`Update`
      (`self.K2_SetActorLocation` (`KismetMathLibrary.VLerp` (`KismetMathLibrary.MakeVector` _returnvalue_x (+ _returnvalue_y 150.0) _returnvalue_z) (`self.PosB`) _curve)))
    (:`Finished`
      (`self.Return From Star`))))

(event `self.ReceiveTick`
  (params (DeltaSeconds :type "Float (single-precision)"))
  (if (`self.IsFollowing`)
    (`SceneComponent.SetVisibility` (`self.StarInMouth`) false true)))

(event `Return From Star`
  (bind (_returnvalue_x _returnvalue_y _returnvalue_z) (`KismetMathLibrary.BreakVector` (`self.K2_GetActorLocation` (`GameplayStatics.GetPlayerPawn` 0))))
  ;[1 1 1] Bird Goes and Gets the Star
  (bind (_direction _curve) (`Timeline|Timeline_0` :!via `ReverseFromEnd`)
    (:`Update`
      (`self.K2_SetActorLocation` (`KismetMathLibrary.VLerp` (`KismetMathLibrary.MakeVector` _returnvalue_x (+ _returnvalue_y 150.0) _returnvalue_z) (`self.PosB`) _curve)))
    (:`Finished`
      (set `self.IsFollowing` true))))

(fn `UserConstructionScript`)