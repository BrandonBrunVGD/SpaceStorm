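; Shield power-up pickup that drifts down along world Z while rotating, using fixed per-tick offsets not scaled by delta time.
; On overlap with a BP_Character whose Shield differs from MaxShield, it refills the shield, adds score and destroys itself.
; A character already at max shield leaves the pickup in place.
; Overlapping a BP_DeathWall also destroys it, without any reward.
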(event `self.ReceiveBeginPlay`)

(event `self.ReceiveActorBeginOverlap`
  (params (OtherActor :type "Actor Object Reference"))
  (bind _as_bp_character (`self.As BP Character`))
  (bind _as_bp_character_2 (`self.As BP Character`))
  (bind _maxshield (`/Game/Ship/BP_Character.MaxShield` _as_bp_character))
  (bind _asbp_character (cast `/Game/Ship/BP_Character` OtherActor)
    (:`then`
      (set `self.As BP Character` _asbp_character)
      (if (not (== (`/Game/Ship/BP_Character.Shield` _as_bp_character) _maxshield))
        (set `/Game/Ship/BP_Character.Shield` _maxshield _as_bp_character)
        (set `/Game/Ship/BP_Character.Score` (+ (`/Game/Ship/BP_Character.Score` _as_bp_character_2) 50) _as_bp_character_2)
        (`self.K2_DestroyActor`)))
    (:`CastFailed`
      (cast `/Game/Blueprints/Bounds/BP_DeathWall` OtherActor)
      (`self.K2_DestroyActor`))))

(event `self.ReceiveTick`
  (params (DeltaSeconds :type "Float (single-precision)"))
  (`self.K2_AddActorWorldOffset` (0.0 0.0 -0.5))
  (`self.K2_AddActorWorldRotation` (struct :`Roll` -0.5)))

(fn `UserConstructionScript`)