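; Player ship for a 2D shooter, handling axis movement, sprite tilt, and single or double bullet fire with a timed reset.
; Overlaps with asteroids, enemies, enemy bullets and rockets drain shield before lives, while boundary overlaps nudge the ship.
; Tick updates shield visuals, game-over and power-up state, and positions a spawned pet beside the ship while it follows.
; BeginPlay detaches the camera so it stays independent of ship movement.
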(event `self.ReceiveBeginPlay`
  (`SceneComponent.K2_DetachFromComponent` (`self.Camera`) "KeepWorld" "KeepWorld" "KeepWorld" true)
  (bind _returnvalue (`|SpawnActorFromClass` "/Game/Blueprints/Pets/BP_Pet.BP_Pet_C" (`KismetMathLibrary.Conv_VectorToTransform` (`SceneComponent.K2_GetComponentLocation` (`self.PaperSprite`))) "Undefined" "MultiplyWithRoot" null (0.0 0.0 0.0) (0.0 0.0 0.0) null))
  (set `self.BP_Pet` _returnvalue))

(event `InputAxis|MovementY`
  (params (AxisValue :type "Float (single-precision)"))
  (`self.K2_AddActorWorldOffset` (`KismetMathLibrary.MakeVector` 0.0 0.0 (* AxisValue (`self.MoveSpeed`)))))

(event `InputAxis|MovementX`
  (params (AxisValue :type "Float (single-precision)"))
  (`self.K2_AddActorWorldOffset` (`KismetMathLibrary.MakeVector` 0.0 (* AxisValue (`self.MoveSpeed`)))))

(event `InputAction|RotationRelease`
  (params (Key :type "Key Structure"))
  (:`Pressed`
    (`SceneComponent.K2_SetWorldRotation` (`self.PaperSprite`) (struct :`Yaw` 45.0) false false))
  (:`Released`
    (`SceneComponent.K2_SetWorldRotation` (`self.PaperSprite`) (struct :`Yaw` 90.0) false false)))

(event `InputAction|Shoot`
  (params (Key :type "Key Structure"))
  (bind _returnvalue (`self.GetTransform`))
  (:`Pressed`
    (switch `int` (`self.FirngModes`)
      (:`Default`
        (`|SpawnActorFromClass` "/Game/Blueprints/Bullet/BP_Bullet.BP_Bullet_C" (`KismetMathLibrary.MakeTransform` (`KismetMathLibrary.MakeVector` (.x (.location _returnvalue)) (.y (.location _returnvalue)) (.z (.location _returnvalue))) (.rotation _returnvalue) (.scale _returnvalue)) "Undefined" "MultiplyWithRoot" null null :!label _label))
      (:`0`
        (goto _label))
      (:`1`
        (`|SpawnActorFromClass` "/Game/Blueprints/Bullet/BP_Bullet.BP_Bullet_C" (`KismetMathLibrary.MakeTransform` (`KismetMathLibrary.MakeVector` (.x (.location _returnvalue)) (- (.y (.location _returnvalue)) 20.0) (.z (.location _returnvalue))) (.rotation _returnvalue) (.scale _returnvalue)) "Undefined" "MultiplyWithRoot" null null)
        (`|SpawnActorFromClass` "/Game/Blueprints/Bullet/BP_Bullet.BP_Bullet_C" (`KismetMathLibrary.MakeTransform` (`KismetMathLibrary.MakeVector` (.x (.location _returnvalue)) (+ (.y (.location _returnvalue)) 20.0) (.z (.location _returnvalue))) (.rotation _returnvalue) (.scale _returnvalue)) "Undefined" "MultiplyWithRoot" null null)))))

(event `DoubleShootTimer`
  (if (!= (`self.FirngModes`) 0)
    (`KismetSystemLibrary.RetriggerableDelay` (`self.PowerUpTime`))
    (set `self.FirngModes` 0)))

(event `self.ReceiveActorBeginOverlap`
  (params (OtherActor :type "Actor Object Reference"))
  (cast `/Game/Blueprints/Asteroids/BP_Asteroid` OtherActor
    (:`then`
      _)
    (:`CastFailed`
      (`self.HandleBounds` OtherActor)
      (cast `/Game/Blueprints/Enemies/UFO/BP_Enemy` OtherActor
        (:`then`
          _)
        (:`CastFailed`
          (cast `/Game/Blueprints/Enemies/BP_EBullet` OtherActor
            (:`then`
              _)
            (:`CastFailed`
              (cast `/Game/Blueprints/Enemies/Rocket/BP_Rocket` OtherActor)))))))
  (if (<= (`self.Shield`) 0.0)
    (`|SpawnActorFromClass` "/Game/FX/ShipHitEffect.ShipHitEffect_C" (`self.GetTransform`) "Undefined" "MultiplyWithRoot" null null)
    (set `self.HitIndicatorColor` false)
    (set `self.Lives` (- (`self.Lives`) 1.0))
    (else
      (set `self.HitIndicatorColor` true)
      (set `self.Shield` (- (`self.Shield`) 1.0))))
  (set `self.DisplayHitIndicator` true))

(event `HandleActivePU`
  (if (== (`self.FirngModes`) 1)
    (set `self.ActivePU` 1)
    (else
      (set `self.ActivePU` 0))))

(event `HandleBounds`
  (params (NewParam :type "Actor Object Reference"))
  (cast `/Game/Blueprints/Bounds/BP_BoundsBottom` NewParam
    (:`then`
      (`self.K2_AddActorWorldOffset` (0.0 0.0 1.0)))
    (:`CastFailed`
      (cast `/Game/Blueprints/Bounds/BP_BoundsTop` NewParam
        (:`then`
          (`self.K2_AddActorWorldOffset` (0.0 0.0 -1.0)))
        (:`CastFailed`
          (cast `/Game/Blueprints/Bounds/BP_BoundsLeft` NewParam
            (:`then`
              (`self.K2_AddActorWorldOffset` (0.0 -1.0 0.0)))
            (:`CastFailed`
              (cast `/Game/Blueprints/Bounds/BP_BoundsRight` NewParam)
              (`self.K2_AddActorWorldOffset` (0.0 1.0 0.0)))))))))

(event `AddStars`
  (params (addingStars :type Integer))
  (set `self.Stars` (+ (`self.Stars`) (`self.StarsAdded`)))
  (set `self.DisplayAddedStars` true))

(event `self.ReceiveTick`
  (params (DeltaSeconds :type "Float (single-precision)"))
  (bind (_returnvalue_x _returnvalue_y _returnvalue_z) (`KismetMathLibrary.BreakVector` (`SceneComponent.K2_GetComponentLocation` (`self.PaperSprite`))))
  (`self.HandleShields/Lives`)
  (`self.HandleActivePU`)
  (if (`/Game/Blueprints/Pets/BP_Pet.IsFollowing` (`self.BP_Pet`))
    (`self.K2_SetActorLocation` (`self.BP_Pet`) (`KismetMathLibrary.MakeVector` _returnvalue_x (+ _returnvalue_y 150.0) _returnvalue_z) false false)))

(event `HandleShields/Lives`
  (bind _shieldglow (`self.ShieldGlow`))
  (bind _shielddisplay (`self.ShieldDisplay`))
  (`SceneComponent.K2_AddLocalRotation` (`self.ShieldDisplay`) (struct :`Pitch` 1.0) false false)
  (if (<= (`self.Lives`) 0.0)
    (set `self.GameOver` true)
    (elif (<= (`self.Shield`) 0.0)
      (`SceneComponent.SetHiddenInGame` _shielddisplay true false)
      (`SceneComponent.SetHiddenInGame` _shieldglow true false)
      (else
        (`SceneComponent.SetHiddenInGame` _shielddisplay false false)
        (`SceneComponent.SetHiddenInGame` _shieldglow false false)))))

(fn `UserConstructionScript`)